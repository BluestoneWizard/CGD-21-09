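; Prototype mirror pawn that the player possesses by interacting with it and rotates in yaw, with the Interact input returning control and view to the character.
; C triggers reverse rotation, while RotateMirror turns forward but has no caller here.
; Both use SetRotationTarget to clamp world yaw to ±75 degrees.
; Timelines feed RInterpTo as delta time, but DefaultRotation becomes the target on the first update, cutting interpolation short.
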(event EventReverseRotateMirror
  (CallFunction|SetRotationTarget (* (Variables|Default|GetRotationAmount) -1.0))
  (bind _value (Timeline|Timeline_0 PlayFromStart)
    (:Update
      (Transformation|SetWorldRotation (Variables|Default|GetMesh) (Math|Rotator|MakeRotator (.Roll (Math|Rotator|BreakRotator (Math|Interpolation|RInterpTo (Variables|Default|GetDefaultRotation) (Variables|Default|GettargetRotation) _value 2.0))) (.Pitch (Math|Rotator|BreakRotator (Math|Interpolation|RInterpTo (Variables|Default|GetDefaultRotation) (Variables|Default|GettargetRotation) _value 2.0))) (.Yaw (Math|Rotator|BreakRotator (Math|Interpolation|RInterpTo (Variables|Default|GetDefaultRotation) (Variables|Default|GettargetRotation) _value 2.0)))) false false)
      (Variables|Default|SetDefaultRotation (Variables|Default|GettargetRotation)))))

(event EventRotateMirror
  (CallFunction|SetRotationTarget (Variables|Default|GetRotationAmount))
  (bind _value (Timeline|Roate PlayFromStart)
    (:Update
      (Transformation|SetWorldRotation (Variables|Default|GetMesh) (Math|Rotator|MakeRotator (.Roll (Math|Rotator|BreakRotator (Math|Interpolation|RInterpTo (Variables|Default|GetDefaultRotation) (Variables|Default|GettargetRotation) _value 2.0))) (.Pitch (Math|Rotator|BreakRotator (Math|Interpolation|RInterpTo (Variables|Default|GetDefaultRotation) (Variables|Default|GettargetRotation) _value 2.0))) (.Yaw (Math|Rotator|BreakRotator (Math|Interpolation|RInterpTo (Variables|Default|GetDefaultRotation) (Variables|Default|GettargetRotation) _value 2.0)))) false false)
      (Variables|Default|SetDefaultRotation (Variables|Default|GettargetRotation)))))

(event EventInteract
  (params (Human%20Char :type Bp%20Base%20Character%20Object%20Reference))
  (bind _returnvalue (Game|GetPlayerController 0))
  ;[1 1 1] Possess this pawn when it is interacted with
  (Variables|Default|SetCharacter Human%20Char)
  (Pawn|Possess _returnvalue self)
  (Game|Player|SetViewTargetwithBlend _returnvalue self 0.0 "VTBlend_Linear" 0.0 false)
  (Variables|Default|SetStartingRotation (Transformation|GetWorldRotation (Variables|Default|GetMesh)))
  (Variables|Default|SetDefaultRotation (Transformation|GetWorldRotation (Variables|Default|GetMesh))))

(event Input|ActionEvents|InputActionInteract
  (params (Key :type Key%20Structure :default "None"))
  (bind _returnvalue (Game|GetPlayerController 0))
  (bind _character (Variables|Default|GetCharacter))
  (:Pressed
    (Pawn|Possess _returnvalue _character)
    (Game|Player|SetViewTargetwithBlend _returnvalue _character 0.0 "VTBlend_Linear" 0.0 false)))

(event Input|KeyboardEvents|C
  (params (Key :type Key%20Structure :default "None"))
  (:Pressed
    (CallFunction|ReverseRotateMirror)))

(fn ConstructionScript)

(fn SetRotationTarget
  (params (Amount :type Float%20%28single-precision%29))
  (bind _defaultrotation (Variables|Default|GetDefaultRotation))
  (bind (_roll _pitch _yaw) (Math|Rotator|BreakRotator _defaultrotation))
  (bind _returnvalue (+ Amount _yaw))
  (if (> _returnvalue 75.0)
    (Variables|Default|SettargetRotation (Math|Rotator|MakeRotator _roll _pitch 75.0))
    (elif (< _returnvalue -75.0)
      (Variables|Default|SettargetRotation (Math|Rotator|MakeRotator _roll _pitch -75.0))
      (else
        (Variables|Default|SettargetRotation (Math|Rotator|MakeRotator _roll _pitch _returnvalue))))))

(fn GetMirrorRef
  (return 0))