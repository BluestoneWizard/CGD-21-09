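; Base box Blueprint with a lid that swings open and closed through Open and Close events.
; Each event plays its own timeline, lerping BoxLid along the shortest path toward the open angle or back to zero rotation.
; Every update lerps from the lid's current world rotation but sets relative rotation, so the motion compounds and mixes coordinate spaces.
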(event Custom|Close
  (bind _value (Timeline|CloseTime Play)
    (:Update
      (Transformation|SetRelativeRotation (Variables|Default|GetBoxLid) (Math|Rotator|Lerp(Rotator) (Transformation|GetWorldRotation (Variables|Default|GetBoxLid)) "0, 0, 0" _value true) false false))))

(event EventOpen
  (bind _value (Timeline|OpenTime Play)
    (:Update
      (Transformation|SetRelativeRotation (Variables|Default|GetBoxLid) (Math|Rotator|Lerp(Rotator) (Transformation|GetWorldRotation (Variables|Default|GetBoxLid)) "-120.000000, 0, 0" _value true) false false))))

(fn ConstructionScript)