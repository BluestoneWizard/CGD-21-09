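; Human player character Blueprint that supports a ghost mechanic and collects crystal fragments.
; Initalize spawns one hidden BP_CharacterBlocking actor, which ghost-blocking events show at the character's location or hide again.
; GhostActivate and GhostDeactivate toggle CanGhostActive, GetGhostSpawnPoint exposes a component's world location, and Interact input calls ActivateInteract.
; Fragments accumulate in CrystalFragments, which GetNumberOfCystalFrag returns whole rather than as a count.
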(event EventGhostActivate
  (Development|PrintString "Active")
  (Variables|Default|SetCanGhostActive true))

(event EventGhostDeactivate
  (Variables|Default|SetCanGhostActive false))

(event EventActivateGhostBlocking
  (Default|SpawntoGame (Variables|Default|GetGhostBlocking) (Transformation|GetActorLocation)))

(event EventDeactivateGhostBlocking
  (Default|HideinWorld (Variables|Default|GetGhostBlocking)))

(event EventInitalize
  (bind _returnvalue (Game|SpawnActorfromClass "/Game/JamieL/Characters/BP_CharacterBlocking.BP_CharacterBlocking_C" (Math|Transform|MakeTransform "0, 0, 0" "0, 0, 0" "1,1,1") "Undefined" 0 0))
  (bind _output_get (Variables|Default|SetGhostBlocking _returnvalue))
  (Default|HideinWorld _output_get))

(event EventAddCrystalFragment
  (params (Fragment :type Crystal%20Fragment%20Object%20Reference))
  (Utilities|Array|Add (Variables|Default|GetCrystalFragments) Fragment))

(event Input|ActionEvents|InputActionInteract
  (params (Key :type Key%20Structure))
  (:Pressed
    (CallFunction|ActivateInteract)))

(fn ConstructionScript)

(fn GetGhostSpawnPoint
  (return (Transformation|GetWorldLocation (Variables|Default|GetGhostSpawnPoint))))

(fn GetNumberOfCystalFrag
  (return (Variables|Default|GetCrystalFragments)))