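; Player controller that lets the player switch possession between a human character and a ghost form.
; On BeginPlay it possesses the level's BP_HumanCharacter and spawns a hidden, non-colliding BP_GhostCharacter.
; ChangeToGhost input, gated by the human's CanGhostActive, reveals the ghost at a spawn point supplied by the human, or hides it and repossesses the human.
; Interact input always forwards to the human, which also receives ghost-blocking messages.
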(event Custom|SpawnGhost
  (bind _returnvalue (Game|SpawnActorfromClass "/Game/JamieL/Characters/Bp_GhostCharacter.BP_GhostCharacter_C" (Math|Transform|MakeTransform "-50.000000, 0, 0" "0, 0, 0" "1,1,1") "AdjustIfPossibleButAlwaysSpawn" 0 0))
  (bind _output_get (Variables|Default|SetGhostCharcter _returnvalue))
  (Collision|SetCollisionEnabled (Variables|/Script/Engine.Character|GetCapsuleComponent _output_get) "NoCollision")
  (Rendering|SetActorHiddenInGame _output_get true)
  (Class|BPIInitalize|Initalize(Message) _output_get))

(event Custom|SpawnHuman
  (bind _outactors (Actor|GetAllActorsOfClass "/Game/JamieL/Characters/BP_HumanCharacter.BP_HumanCharacter_C"))
  (Pawn|Possess (Utilities|Array|Get(acopy) _outactors))
  (bind _output_get (Variables|Default|SetHumanCharacter (Utilities|Array|Get(acopy) _outactors)))
  (Class|BPIInitalize|Initalize(Message) _output_get))

(event EventBeginPlay
  (CallFunction|SpawnHuman)
  (CallFunction|SpawnGhost))

(event Input|ActionEvents|InputActionChangeToGhost
  (params (Key :type Key%20Structure :default "None"))
  (:Pressed
    (if (== (Pawn|GetControlledPawn) (Variables|Default|GetHumanCharacter))
      (if (Math|Boolean|Equal(Boolean) (Variables|/Game/JamieL/Characters/BP_HumanCharacter.BP_HumanCharacter_C|GetCanGhostActive (Variables|Default|GetHumanCharacter)) true)
        (CallFunction|ChangetoGhost))
      (else
        (CallFunction|ChangetoHuman)
        (Class|BPIHuman|DeactivateGhostBlocking(Message) (Variables|Default|GetHumanCharacter))))))

(event Input|ActionEvents|InputActionInteract
  (params (Key :type Key%20Structure :default "None"))
  (:Pressed
    (Default|ActivateInteract (Variables|Default|GetHumanCharacter))))

(fn ConstructionScript)

(fn ChangetoGhost
  (bind _returnvalue (Pawn|GetControlledPawn))
  (bind _ghostcharcter (Variables|Default|GetGhostCharcter))
  (bind _location (Class|BPIHuman|GetGhostSpawnPoint(Message) _returnvalue))
  (Class|BPIHuman|ActivateGhostBlocking(Message) _returnvalue)
  (Transformation|SetActorLocationAndRotation (Variables|Default|GetGhostCharcter) _location (Pawn|GetControlRotation _returnvalue :!class /Script/Engine.Pawn))
  (Collision|SetCollisionEnabled (Variables|/Script/Engine.Character|GetCapsuleComponent (Variables|Default|GetGhostCharcter)) "QueryAndPhysics")
  (Rendering|SetActorHiddenInGame _ghostcharcter false)
  (Pawn|Possess _ghostcharcter))

(fn ChangetoHuman
  (Collision|SetCollisionEnabled (Variables|/Script/Engine.Character|GetCapsuleComponent (Variables|Default|GetGhostCharcter)) "NoCollision")
  (Rendering|SetActorHiddenInGame (Variables|Default|GetGhostCharcter) true)
  (Pawn|Possess (Variables|Default|GetHumanCharacter)))