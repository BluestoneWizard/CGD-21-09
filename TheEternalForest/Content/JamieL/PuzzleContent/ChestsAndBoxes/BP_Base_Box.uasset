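; Base puzzle box actor with a hinged lid, a child-actor lock and four journal notes that carry its number code.
; Initalize messages the lock, while Open and Close rotate the lid through timelines using RInterpTo and a rotator lerp.
; GenerateNotesForBox spawns the four notes at the box and ClearNotes destroys them.
; SetCode stores the code and passes one digit to each note by array index.
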(event EventInitalize
  (Class|BPIInitalize|Initalize(Message) (Variables|/Script/Engine.ChildActorComponent|GetChildActor (Variables|Default|GetLock))))

(event EventOpen
  (bind _boxlid (Variables|Default|GetBoxLid))
  (bind _returnvalue (Transformation|GetWorldRotation _boxlid))
  (bind (_roll _pitch _yaw) (Math|Rotator|BreakRotator _returnvalue))
  ;[1 1 1] Open and close box
  (bind _value (Timeline|OpenTime PlayFromStart)
    (:Update
      (Transformation|SetWorldRotation (Variables|Default|GetBoxLid) (Math|Interpolation|RInterpTo _returnvalue (Math|Rotator|MakeRotator -1.2e+02 _pitch _yaw) (Utilities|Time|GetWorldDeltaSeconds) 2.0) false false))))

(event EventClose
  ;[1 1 1] Open and close box
  (bind _value (Timeline|CloseTime PlayFromStart)
    (:Update
      (Transformation|SetRelativeRotation (Variables|Default|GetBoxLid) (Math|Rotator|Lerp(Rotator) (Transformation|GetWorldRotation (Variables|Default|GetBoxLid)) "0, 0, 0" _value true) false false))))

(event EventSetCode
  (params (Code :type Codes%20Structure))
  (Variables|Default|SetCode Code)
  (Notes|SetValueonNotes))

(fn ConstructionScript)

(fn GenerateNotesforBox
  (if (Utilities|Array|IsValidIndex (Variables|Notes|GetNotes))
    (Development|PrintString "Notes Already Exist" true true "(R=1.000000,G=0.000000,B=0.000000,A=1.000000)" 5.0)
    (else
      (for _index (range 0 3)
        (bind _returnvalue (Game|SpawnActorfromClass "/Game/JamieL/Journal/NumberCode_Box_Journal.NumberCode_Box_Journal_C" (Transformation|GetActorTransform) "Undefined" 0 0))
        (Utilities|Array|Add (Variables|Notes|GetNotes) _returnvalue)))))

(fn ClearNotes
  (bind _notes (Variables|Notes|GetNotes))
  (if (Utilities|Array|IsValidIndex _notes)
    (for _array_element _notes
      (Actor|DestroyActor _array_element))
    (Utilities|Array|Clear (Variables|Notes|GetNotes))
    (else
      (Development|PrintString "No Notes" true true "(R=1.000000,G=0.000000,B=0.027472,A=1.000000)" 5.0))))

(fn SetValueonNotes
  (for (_array_element _array_index) (Variables|Notes|GetNotes)
    ;[1 1 1] Finds the index the number should be
    (if (== _array_index 0)
      ;[1 1 1] Sets the Value of the Node
      (Default|SetNoteValue _array_element (.Number1 (Utilities|Struct|BreakCodes (Variables|Default|GetCode))) 0 (Variables|BoxSettings|GetBox))
      (elif (== _array_index 1)
        (Default|SetNoteValue _array_element (.Number2 (Utilities|Struct|BreakCodes (Variables|Default|GetCode))) 1 (Variables|BoxSettings|GetBox))
        (elif (== _array_index 2)
          (Default|SetNoteValue _array_element (.Number3 (Utilities|Struct|BreakCodes (Variables|Default|GetCode))) 2 (Variables|BoxSettings|GetBox))
          (elif (== _array_index 3)
            (Default|SetNoteValue _array_element (.Nymber4 (Utilities|Struct|BreakCodes (Variables|Default|GetCode))) 3 (Variables|BoxSettings|GetBox))
            (else
              (Development|PrintString "Error"))))))))