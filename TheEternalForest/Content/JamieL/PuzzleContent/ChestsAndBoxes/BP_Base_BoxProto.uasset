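; Prototype base Blueprint for a puzzle box or chest with a hinged lid and a linked code note, though none of its event logic is wired to run.
; Disconnected timelines would swing the lid open with RInterpTo on pitch and close it with a rotator lerp.
; Another orphaned chain would build a placeholder all-zero code, write it to the note's text, and copy the lid's material onto the note.
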(fn ConstructionScript)