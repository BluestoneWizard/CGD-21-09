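; BP_Leaver is an interactable puzzle lever that swings its stick and opens a linked door.
; Each Interact alternates through a FlipFlop between playing and reversing the LeverMove timeline, which lerps Stick's relative rotation from StartingLocation toward a direction combining start and target forward vectors.
; The timeline's Finished event calls Open on BPDoor, while the BPDoor2 Open call is unconnected and never runs.
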(event EventInteract
  (params (Human%20Char :type Bp%20Base%20Character%20Object%20Reference))
  (Utilities|FlowControl|FlipFlop
    (:A
      (bind _value (Timeline|LeverMove PlayFromStart)
        (:Update
          (Transformation|SetRelativeRotation (Variables|Default|GetStick) (Math|Rotator|Lerp(Rotator) (Variables|Default|GetStartingLocation) (Math|Conversions|RotationFromXVector (+ (Math|Rotator|GetRotationXVector (Variables|Default|GetStartingLocation)) (Math|Rotator|GetRotationXVector (Variables|Default|GetTargetLocation)))) _value) false false))
        (:Finished
          (Default|Open (Variables|Default|GetBP_Door)))))
    (:B
      (Timeline|LeverMove ReverseFromEnd))))

(fn ConstructionScript)