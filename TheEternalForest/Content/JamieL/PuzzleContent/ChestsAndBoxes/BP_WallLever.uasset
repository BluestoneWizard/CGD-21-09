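; BP_WallLever is an interactable wall lever that slides its handle downward and announces its activation through an event dispatcher.
; Interact drives a LeverMove timeline that lerps the handle's world location, calling LeverActivated when the pull finishes.
; Deactivate clears the Activated flag and reverses the timeline, with DoOnce gates blocking repeat triggers until the return completes.
; An interaction component highlights the base mesh on request.
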(event Custom|Deactivate
  (bind _leverhandle (Variables|Default|GetLeverHandle))
  (bind _returnvalue (Transformation|GetWorldLocation _leverhandle))
  (Utilities|FlowControl|DoOnce false :!label _label
    (:Completed
      (Variables|Default|SetActivated? false)
      (bind _value (Timeline|LeverMove ReverseFromEnd)
        (:Update
          (Transformation|SetWorldLocation (Variables|Default|GetLeverHandle) (Math|Vector|Lerp(Vector) (Variables|Default|GetWorldLocation) (Variables|Default|GetTargetLocation) _value) false false))
        (:Finished
          (if (Variables|Default|GetActivated?)
            (Default|CallLeverActivated self)
            (else
              (Utilities|FlowControl|Sequence
                (:then_0
                  (Utilities|FlowControl|DoOnce false) ; enters at Reset
                )
                (:then_1
                  (goto _label Reset))))))))))

(event EventInteract
  (params (Human%20Char :type Bp%20Base%20Character%20Object%20Reference))
  (bind _leverhandle (Variables|Default|GetLeverHandle))
  (bind _returnvalue (Transformation|GetWorldLocation _leverhandle))
  (if (not (Variables|Default|GetActivated?))
    (Utilities|FlowControl|DoOnce false :!label _label
      (:Completed
        (Variables|Default|SetActivated? true)
        (Variables|Default|SetWorldLocation _returnvalue)
        (Variables|Default|SetTargetLocation (- _returnvalue "0, 0,30.000000"))
        (bind _value (Timeline|LeverMove PlayFromStart)
          (:Update
            (Transformation|SetWorldLocation (Variables|Default|GetLeverHandle) (Math|Vector|Lerp(Vector) (Variables|Default|GetWorldLocation) (Variables|Default|GetTargetLocation) _value) false false))
          (:Finished
            (if (Variables|Default|GetActivated?)
              (Default|CallLeverActivated self)
              (else
                (Utilities|FlowControl|Sequence
                  (:then_0
                    (goto _label Reset))
                  (:then_1
                    (Utilities|FlowControl|DoOnce false) ; enters at Reset
                  ))))))))))

(event EventHiglightMesh
  (params (Higlight :type Boolean))
  (Default|HighlightMesh (Variables|Default|GetInteraction_Component) Higlight (Utilities|Array|MakeArray (Variables|Default|GetBase))))

(fn ConstructionScript)