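; BP_Mirror is an interactable puzzle mirror pawn that the player takes control of and rotates.
; Interacting hides the character, disables its collision and possesses the mirror, and pressing Interact again restores the character.
; Left and right inputs play DoOnce-gated timelines that apply yaw by value deltas, while LimitMirror clamps it between minimum and maximum rotation.
; Highlighting is passed to the interaction component.
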(event EventHiglightMesh
  (params (Higlight :type Boolean))
  (Default|HighlightMesh (Variables|Default|GetInteraction_Component) Higlight (Utilities|Array|MakeArray (Variables|Default|GetMirror) (Variables|Default|GetSM_Mirror_Stand))))

(event EventInteract
  (params (Human%20Char :type Bp%20Base%20Character%20Object%20Reference) (Pawn :type Pawn%20Object%20Reference))
  (bind _returnvalue (Game|GetPlayerController 0))
  ;[1 1 1] Possess this pawn when it is interacted with
  (bind _output_get (Variables|Default|SetCharacter Human%20Char))
  (Rendering|SetActorHiddenInGame _output_get true)
  (bind _humancharacter (Class|BPIHuman|GetHumanCharacter(Message) Human%20Char))
  (Default|SetCollision _humancharacter false)
  (Pawn|Possess _returnvalue self)
  (Game|Player|SetViewTargetwithBlend _returnvalue self 0.0 "VTBlend_Linear" 0.0 false))

(event Input|ActionEvents|InputActionInteract
  (params (Key :type Key%20Structure :default "None"))
  (bind _returnvalue (Game|GetPlayerController 0))
  (bind _character (Variables|Default|GetCharacter))
  ;[1 1 1] Is fired when the player uses the interact key and then possesses the character again
  (:Pressed
    (Pawn|Possess _returnvalue _character)
    (Game|Player|SetViewTargetwithBlend _returnvalue _character 0.0 "VTBlend_Linear" 0.0 false)
    (Rendering|SetActorHiddenInGame _character false)
    (bind _humancharacter (Class|BPIHuman|GetHumanCharacter(Message) (Variables|Default|GetCharacter)))
    (Default|SetCollision _humancharacter true)))

(event Input|ActionEvents|InputActionMoveObjecttLeft
  (params (Key :type Key%20Structure :default "None"))
  (:Pressed
    (Utilities|FlowControl|DoOnce false :!label _label
      (:Completed
        (bind _value (Timeline|ReverseRotate PlayFromStart)
          (:Update
            (bind _can_rotate_ (CallFunction|LimitMirror))
            (if _can_rotate_
              (Transformation|AddRelativeRotation (Variables|Default|GetMirror) (Math|Rotator|MakeRotator 0.0 0.0 (* (* (- _value (Variables|Default|GetPreviousValue)) (Variables|Default|GetRotationAmount)) -1.0)) false false)
              (Variables|Default|SetPreviousValue _value)))
          (:Finished
            (Variables|Default|SetPreviousValue 0.0)
            (goto _label Reset)))))))

(event Input|ActionEvents|InputActionMoveObjectRight
  (params (Key :type Key%20Structure :default "None"))
  (:Pressed
    (Utilities|FlowControl|DoOnce false :!label _label
      (:Completed
        (bind _value (Timeline|Roate PlayFromStart)
          (:Update
            (bind _can_rotate_ (CallFunction|LimitMirror))
            (if _can_rotate_
              (Transformation|AddRelativeRotation (Variables|Default|GetMirror) (Math|Rotator|MakeRotator 0.0 0.0 (* (- _value (Variables|Default|GetPreviousValue)) (Variables|Default|GetRotationAmount))) false false)
              (Variables|Default|SetPreviousValue _value)))
          (:Finished
            (Variables|Default|SetPreviousValue 0.0)
            (goto _label Reset)))))))

(fn ConstructionScript)

(fn LimitMirror
  (bind _mirror (Variables|Default|GetMirror))
  (bind _relativerotation (Variables|/Script/Engine.SceneComponent|GetRelativeRotation _mirror))
  (bind _yaw (Math|Rotator|BreakRotator _relativerotation))
  (if (> _yaw (Variables|Default|GetMaxRotation))
    (Transformation|SetRelativeRotation (Variables|Default|GetMirror) (Math|Rotator|MakeRotator 0.0 0.0 (- (Variables|Default|GetMaxRotation) 0.001)) false false)
    (elif (< _yaw (Variables|Default|GetMinRotation))
      (Transformation|SetRelativeRotation (Variables|Default|GetMirror) (Math|Rotator|MakeRotator 0.0 0.0 (+ (Variables|Default|GetMinRotation) 0.001)) false false)
      (else
        (return true))))
  (return false))

(fn GetMirrorRef
  (return self))