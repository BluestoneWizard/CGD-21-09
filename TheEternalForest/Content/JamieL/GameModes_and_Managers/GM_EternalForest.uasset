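; GM_EternalForest is the game mode for the Eternal Forest that sets up and routes the main player UI.
; On BeginPlay it creates the main game UI widget, initializes its message state, adds it to the viewport and caches references to its pause menu and options screen.
; A SwitchGameModeUI event forwards screen selections to that widget, while PostLogin and logout events maintain a list of player controllers.
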(event EventSwitchGameModeUI
  (params (Selection :type GameUI%20Enum :default "NewEnumerator7"))
  (Class|BPIUI|SwitchUI(Message) (Variables|UI|GetMainPlayerUI) Selection))

(event EventBeginPlay
  (CallFunction|SetUpUI))

(event EventPostLogin
  (params (NewPlayer :type Player%20Controller%20Object%20Reference))
  (Utilities|Array|Add (Variables|Default|GetPlayerController) NewPlayer))

(event EventOnLogout
  (params (ExitingController :type Controller%20Object%20Reference))
  (Utilities|Array|RemoveItem (Variables|Default|GetPlayerController) (.AsPC%20Player (Utilities|Casting|CastToPC_Player ExitingController))))

(fn ConstructionScript)

(fn SetUpUI
  (bind _returnvalue (UserInterface|CreateWidget "/Game/JamieL/UI/GameUI/UI_MainGameUI.UI_MainGameUI_C"))
  (bind _output_get (Variables|UI|SetMainPlayerUI _returnvalue))
  (Class|BPIUI|InitUI(Message) _output_get "NewEnumerator7")
  (UserInterface|Viewport|AddtoViewport _output_get 0)
  (Variables|UI|SetUI_PauseMenu (Variables|/Game/JamieL/UI/GameUI/UI_MainGameUI.UI_MainGameUI_C|GetUI_PauseMenu _output_get))
  (Variables|UI|SetOptionsUI (Variables|/Game/JamieL/UI/GameUI/UI_MainGameUI.UI_MainGameUI_C|GetUI_OptionsScreen _output_get)))