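; Base box Blueprint with a hinged lid and a linked note that shows the box's four-number code.
; Open and Close events play timelines that rotate the lid, using RInterpTo toward a fixed roll to open and a rotator lerp to close.
; SetCode joins the numbers into OwnCode, writes it on the note, and gives the note the lid's material so the two match.
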(event EventOpen
  (bind _boxlid (Variables|Default|GetBoxLid))
  (bind _returnvalue (Transformation|GetWorldRotation _boxlid))
  (bind (_roll _pitch _yaw) (Math|Rotator|BreakRotator _returnvalue))
  (bind _value (Timeline|OpenTime PlayFromStart)
    (:Update
      (Transformation|SetWorldRotation (Variables|Default|GetBoxLid) (Math|Interpolation|RInterpTo _returnvalue (Math|Rotator|MakeRotator -1.2e+02 _pitch _yaw) (Utilities|Time|GetWorldDeltaSeconds) 2.0) false false))))

(event EventClose
  (bind _value (Timeline|CloseTime PlayFromStart)
    (:Update
      (Transformation|SetRelativeRotation (Variables|Default|GetBoxLid) (Math|Rotator|Lerp(Rotator) (Transformation|GetWorldRotation (Variables|Default|GetBoxLid)) "0, 0, 0" _value true) false false))))

(event EventSetCode
  (params (SetCode :type Codes%20Structure))
  (bind _output_get (Variables|Default|SetOwn%20Code (Utilities|String|Append (Utilities|String|ToString(Integer) (.number1 SetCode)) (Utilities|String|ToString(Integer) (.number2 SetCode)) (Utilities|String|ToString(Integer) (.number3 SetCode)) (Utilities|String|ToString(Integer) (.nymber4 SetCode)))))
  (Rendering|Components|TextRender|SetText (Variables|/Game/JamieD/Tumbler/B_BaseNote.B_BaseNote_C|GetTextRender (Variables|Default|GetNote)) (Utilities|Text|ToText(String) _output_get))
  (Rendering|Material|SetMaterial (Variables|/Game/JamieD/Tumbler/B_BaseNote.B_BaseNote_C|GetNote (Variables|Default|GetNote)) 0 (Rendering|Material|GetMaterial (Variables|Default|GetBoxLid) 0)))

(fn ConstructionScript)